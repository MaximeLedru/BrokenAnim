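; AI pawn Blueprint that patrols the level by wandering between target points.
; On BeginPlay it runs Patrouiller, which picks a random TargetPoint tagged "Monstre" and moves there with AIMoveTo.
; Whether the move succeeds or fails, it waits a random few seconds and calls itself again, forming an endless patrol loop.
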(event Custom|Patrouiller
  (bind _outactors (Actor|GetAllActorsOfClasswithTag "/Script/Engine.TargetPoint" "Monstre"))
  (AI|AIMoveTo self (Transformation|GetActorLocation (Utilities|Array|Get(acopy) _outactors (Math|Random|RandomInteger (Utilities|Array|Length _outactors)))) 0 5.0 false
    (:OnSuccess
      _)
    (:OnFail
      _))
  (Utilities|FlowControl|Delay (Math|Random|RandomFloatinRange 2.0 8.0))
  (CallFunction|Patrouiller))

(event EventBeginPlay
  (CallFunction|Patrouiller))

(event Collision|EventActorBeginOverlap
  (params (OtherActor :type Actor%20Object%20Reference)))

(event EventTick
  (params (DeltaSeconds :type Float%20%28single-precision%29)))

(fn ConstructionScript)